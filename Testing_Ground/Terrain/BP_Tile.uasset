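; BP_Tile is a terrain tile for infinite level generation, with an Arrow component that supplies an attach point transform.
; Player overlap with LevelLockBox turns the Barrier green and disables its collision.
; Leaving that box turns the Barrier red and solid again, then asks InfiniteTerrainGameMode to create a tile and update the current transform.
; The tile destroys itself when the player leaves LevelDestroyBox.
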(event OnComponentBeginOverlap(LevelLockBox)
  (params (OverlappedComponent :type Primitive%20Component%20Object%20Reference) (OtherActor :type Actor%20Object%20Reference) (OtherComp :type Primitive%20Component%20Object%20Reference) (OtherBodyIndex :type Integer) (bFromSweep :type Boolean) (SweepResult :type Hit%20Result%20Structure%20%28by%20ref%29))
  (if (== (Game|Player|GetPlayerPawn 0) OtherActor)
    (CallFunction|UnlockLevel)))

(event OnComponentEndOverlap(LevelDestroyBox)
  (params (OverlappedComponent :type Primitive%20Component%20Object%20Reference) (OtherActor :type Actor%20Object%20Reference) (OtherComp :type Primitive%20Component%20Object%20Reference) (OtherBodyIndex :type Integer))
  (if (== (Game|Player|GetPlayerPawn 0) OtherActor)
    (CallFunction|DestroyTile)))

(event OnComponentEndOverlap(LevelLockBox)
  (params (OverlappedComponent :type Primitive%20Component%20Object%20Reference) (OtherActor :type Actor%20Object%20Reference) (OtherComp :type Primitive%20Component%20Object%20Reference) (OtherBodyIndex :type Integer))
  (if (== (Game|Player|GetPlayerPawn 0) OtherActor)
    (CallFunction|LockLevel)
    (bind _asinfinite_terrain_game_mode (Utilities|Casting|CastToInfiniteTerrainGameMode (Game|GetGameMode)))
    (Default|CreateTileandUpdateCurrentTransform _asinfinite_terrain_game_mode)))

(event EventBeginPlay)

(event Collision|EventActorBeginOverlap
  (params (OtherActor :type Actor%20Object%20Reference)))

(event EventTick
  (params (DeltaSeconds :type Float%20%28single-precision%29)))

(fn ConstructionScript)

(fn GetAttachPoint
  (return (Transformation|GetWorldTransform (Variables|Default|GetArrow))))

(fn UnlockLevel
  (Rendering|Material|SetMaterial (Variables|Default|GetBarrier) 0 "/Game/Dynamic/Terrain/GreenBarrier.GreenBarrier")
  (Collision|SetCollisionEnabled (Variables|Default|GetBarrier) "NoCollision"))

(fn LockLevel
  (Rendering|Material|SetMaterial (Variables|Default|GetBarrier) 0 "/Game/Dynamic/Terrain/RedBarrier.RedBarrier")
  (Collision|SetCollisionEnabled (Variables|Default|GetBarrier) "QueryAndPhysics"))

(fn DestroyTile
  (Actor|DestroyActor))