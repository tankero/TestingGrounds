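; AI controller for guard NPCs that runs the GuardBehavior tree with the PatrolData blackboard.
; AI perception sets any successfully sensed actor without the "NPC" tag as the target, stored under the FocalPointKey blackboard key.
; Helper functions set or clear that target and check whether it is dead.
; FindPatrolRoute does nothing, as its first-waypoint logic is disconnected.
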(event OnTargetPerceptionUpdated(AIPerception)
  (params (Actor :type Actor%20Object%20Reference) (Stimulus :type AI%20Stimulus%20Structure))
  (if (not (Actor|ActorHasTag Actor "NPC"))
    (if (.bsuccessfullysensed Stimulus)
      (CallFunction|SetTarget Actor))))

(event EventBeginPlay
  (bind _blackboardcomponent (Class|AIController|UseBlackboard "/Game/Dynamic/Character/AI/PatrolData.PatrolData"))
  (AI|RunBehaviorTree "/Game/Dynamic/Character/AI/GuardBehavior.GuardBehavior")
  (Variables|Default|SetBlackboard%20Component _blackboardcomponent))

(fn ConstructionScript)

(fn FindPatrolRoute
  (params (Blackboard :type Blackboard%20Component%20Object%20Reference)))

(fn SetTarget
  (params (ObjectValue :type Object%20Object%20Reference))
  (AI|Components|Blackboard|SetValueasObject (Variables|Default|GetBlackboard%20Component) (Variables|Default|GetFocalPointKey) ObjectValue))

(fn ClearTarget
  (AI|Components|Blackboard|ClearValue (Variables|Default|GetBlackboard%20Component) (Variables|Default|GetFocalPointKey)))

(fn IsTargetDead
  (bind _ascharacter (Utilities|Casting|CastToCharacter (AI|Components|Blackboard|GetValueasObject (Variables|Default|GetBlackboard%20Component) (Variables|Default|GetFocalPointKey))))
  (return (Default|IsDead _ascharacter)))