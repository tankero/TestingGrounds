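; AI controller for guard NPCs that runs the guard behavior tree on the patrol blackboard.
; On begin play it starts the tree and caches the blackboard component.
; Perception updates set the focal point key to sensed actors not tagged NPC and clear it when sensing fails.
; FindPatrolRoute is an empty stub, with disconnected logic for writing the first patrol point as the waypoint.
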(event OnTargetPerceptionUpdated(AIPerception)
  (params (Actor :type Actor%20Object%20Reference) (Stimulus :type AI%20Stimulus%20Structure))
  (bind _blackboard_component (Variables|Default|GetBlackboard%20Component))
  (bind _focalpointkey (Variables|Default|GetFocalPointKey))
  (if (not (Actor|ActorHasTag Actor "NPC"))
    (if (.bsuccessfullysensed Stimulus)
      (AI|Components|Blackboard|SetValueasObject _blackboard_component _focalpointkey Actor)
      (else
        (AI|Components|Blackboard|ClearValue _blackboard_component _focalpointkey)))))

(event EventBeginPlay
  (bind _blackboardcomponent (Class|AIController|UseBlackboard "/Game/Dynamic/NPC/AI/PatrolData.PatrolData"))
  (AI|RunBehaviorTree "/Game/Dynamic/NPC/AI/GuardBehavior.GuardBehavior")
  (Variables|Default|SetBlackboard%20Component _blackboardcomponent))

(fn ConstructionScript)

(fn FindPatrolRoute
  (params (Blackboard :type Blackboard%20Component%20Object%20Reference)))